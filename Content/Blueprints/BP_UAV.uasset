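; BP_UAV is an input-driven UAV Blueprint that hands flight control to a FlightDynamics object.
; Throttle, Pitch, Roll and Yaw axis events each write their raw value straight to the matching FlightDynamics input.
; A disconnected leftover chain would accumulate and clamp a throttle value but never runs, and the construction script is empty.
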(event Input|AxisEvents|InputAxisThrottle
  (params (AxisValue :type Float%20%28single-precision%29))
  (Variables|/Script/UAVSimulator.FlightDynamicsComponent|SetThrottleInput (Variables|Default|GetFlightDynamics) AxisValue))

(event Input|AxisEvents|InputAxisPitch
  (params (AxisValue :type Float%20%28single-precision%29))
  (Variables|/Script/UAVSimulator.FlightDynamicsComponent|SetPitchInput (Variables|Default|GetFlightDynamics) AxisValue))

(event Input|AxisEvents|InputAxisRoll
  (params (AxisValue :type Float%20%28single-precision%29))
  (Variables|/Script/UAVSimulator.FlightDynamicsComponent|SetRollInput (Variables|Default|GetFlightDynamics) AxisValue))

(event Input|AxisEvents|InputAxisYaw
  (params (AxisValue :type Float%20%28single-precision%29))
  (Variables|/Script/UAVSimulator.FlightDynamicsComponent|SetYawInput (Variables|Default|GetFlightDynamics) AxisValue))

(fn ConstructionScript)